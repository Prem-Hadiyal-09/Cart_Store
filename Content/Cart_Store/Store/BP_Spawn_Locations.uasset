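; BP_Spawn_Locations is a store spawn point that fills its Child Actor component with a random product.
; SetUpProduct picks a random row from the Products_List data table and sets the child actor class to that row's ProductClass.
; It then casts the spawned actor to BP_Product_Base and passes it the row name through SetData.
; An unconnected branch that applies SetData to all matching products never runs.
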(event Custom|Set%20Up%20Product
  (bind _outrownames (DataTable|GetDataTableRowNames "/Game/Cart_Store/Store/Product/Products_List.Products_List"))
  (bind _output_get (Variables|Default|SetRow%20Name (.OutItem (Utilities|Array|Random _outrownames))))
  (bind _returnvalue (Utilities|GetDataTableRow "/Game/Cart_Store/Store/Product/Products_List.Products_List" _output_get)
    (:then
      (ChildActorComponent|SetChildActorClass (Variables|Default|GetChildActor) (Utilities|Struct|BreakProduct_DATA _returnvalue))
      (bind _asbp_product_base (Utilities|Casting|CastToBP_Product_Base (Variables|/Script/Engine.ChildActorComponent|GetChildActor (Variables|Default|GetChildActor))))
      (Default|SetData _asbp_product_base (Variables|Default|GetRow%20Name)))))

(fn ConstructionScript)