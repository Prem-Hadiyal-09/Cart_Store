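; Base VR grabbable store product that shows its info on a floating UI widget while held.
; The construction script finds its row in Products_List by matching ProductClass to its own class.
; On grab it passes that RowName to the VR game mode's DisplayProductUI and shows the widget.
; A looping timer keeps the widget above the mesh facing the player camera until drop hides it and clears the timer.
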(event OnGrabbed(VRGrabComponent)
  ;[0 0 0 0.5] Grab On Display UI
  (Utilities|FlowControl|Delay 0.05)
  (Default|DisplayProductUI (Variables|Default|GetVR%20Game%20Mode) (Variables|Default|GetRow%20Name))
  (Rendering|SetVisibility (Variables|Default|GetWidget) true false)
  (bind _returnvalue (Utilities|Time|SetTimerbyEvent (delegate Custom|TimerEvent) 0.01 true))
  (Variables|Default|SetTimer%20By%20Event _returnvalue))

(event OnDropped(VRGrabComponent)
  ;[0 0 0 0.5] Drop Grab
  (Rendering|SetVisibility (Variables|Default|GetWidget) false false)
  (Utilities|Time|ClearandInvalidateTimerbyHandle (Variables|Default|GetTimer%20By%20Event)))

(event Custom|TimerEvent
  ;[0 0 0 0.5] Grab On Display UI
  (Utilities|FlowControl|Sequence
    (:then_0
      (Transformation|SetWorldLocation (Variables|Default|GetWidget) (+ (Transformation|GetWorldLocation (Variables|Default|GetStaticMesh)) "0.000000,0.000000,40.000000") false true))
    (:then_1
      (Transformation|SetWorldRotation (Variables|Default|GetWidget) (Math|Rotator|FindLookatRotation (Transformation|GetWorldLocation (Variables|Default|GetWidget)) (Camera|GetCameraLocation (Game|GetPlayerCameraManager 0))) false true))))

(event EventBeginPlay
  (bind _asmy_vr_game_mode (Utilities|Casting|CastToMy_VR_GameMode (Game|GetGameMode)))
  (Variables|Default|SetVR%20Game%20Mode _asmy_vr_game_mode))

(fn ConstructionScript
  (bind _outrownames (DataTable|GetDataTableRowNames "/Game/Cart_Store/Store/Product/Products_List.Products_List"))
  (for _array_element _outrownames
    (bind _returnvalue (Utilities|GetDataTableRow "/Game/Cart_Store/Store/Product/Products_List.Products_List" _array_element)
      (:then
        (if (== (.ProductClass (Utilities|Struct|BreakProduct_DATA _returnvalue)) (Utilities|GetClass self))
          (Variables|Default|SetRow%20Name _array_element))))))

(fn SetData
  (params (Row%20Name :type Name))
  (bind _output_get (Variables|Default|SetRow%20Name Row%20Name))
  (return _output_get))