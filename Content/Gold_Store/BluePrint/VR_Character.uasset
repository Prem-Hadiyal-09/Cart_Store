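; VR player character with smooth locomotion, jump, navmesh-checked arc teleport, grabbing and animated hands.
; Either hand grabs one VRGrabComponent via sphere trace, swapping the opposite hand for a controller model with a widget laser.
; That hand's teleport input then clicks UI; otherwise it previews a predicted projectile path with spawned mesh dots and a ring, teleporting on release.
; Point and grasp inputs drive hand AnimBP pose alphas, while looping timers resize the lasers.
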(event Custom|UngrabAll
  (Utilities|FlowControl|Sequence
    (:then_0
      (bind _lefthandheldcomponent (Variables|Default|GetLeftHandHeldComponent)
        (:then
          (bind _breleased (Default|TryRelease _lefthandheldcomponent))
          (if _breleased
            (Variables|Default|SetLeftHandHeldComponent 0)
            (Variables|Default|SetGrabComponet 0)
            (Components|Activation|Deactivate (Variables|Default|GetWidgetInteractionRight))
            (Rendering|SetVisibility (Variables|Default|GetXRDeviceVisualizationRight) false false)
            (Rendering|SetVisibility (Variables|Default|GetRightHand) true false)))
        (:else)))
    (:then_1
      (bind _righthandheldcomponent (Variables|Default|GetRightHandHeldComponent)
        (:then
          (bind _breleased_2 (Default|TryRelease _righthandheldcomponent))
          (if _breleased_2
            (Variables|Default|SetRightHandHeldComponent 0)
            (Variables|Default|SetGrabComponet 0)
            (Components|Activation|Deactivate (Variables|Default|GetWidgetInteractionLeft))
            (Rendering|SetVisibility (Variables|Default|GetXRDeviceVisualizationLeft) false false)
            (Rendering|SetVisibility (Variables|Default|GetLeftHand) true false)))
        (:else)))))

(event Input|EnhancedActionEvents|EnhancedInputActionVR_Look
  (params (ActionValue :type Vector%202D%20Structure) (ElapsedSeconds :type Float%20%28double-precision%29) (TriggeredSeconds :type Float%20%28double-precision%29) (InputAction :type Input%20Action%20Object%20Reference :default "/Game/Gold_Store/Input/Controlls/VR_Look.VR_Look"))
  (Pawn|Input|AddControllerYawInput (.x ActionValue))
  (Pawn|Input|AddControllerPitchInput (.y ActionValue)))

(event Input|EnhancedActionEvents|EnhancedInputActionVR_Move
  (params (ActionValue :type Vector%202D%20Structure) (ElapsedSeconds :type Float%20%28double-precision%29) (TriggeredSeconds :type Float%20%28double-precision%29) (InputAction :type Input%20Action%20Object%20Reference :default "/Game/Gold_Store/Input/Controlls/VR_Move.VR_Move"))
  (Pawn|Input|AddMovementInput (Math|Vector|GetRightVector (Variables|Default|GetCamera)) (.x ActionValue) false)
  (Pawn|Input|AddMovementInput (Math|Vector|GetForwardVector (Variables|Default|GetCamera)) (.y ActionValue) false))

(event Input|EnhancedActionEvents|EnhancedInputActionVR_Teleport_Right
  (params (ActionValue :type Boolean) (ElapsedSeconds :type Float%20%28double-precision%29) (TriggeredSeconds :type Float%20%28double-precision%29) (InputAction :type Input%20Action%20Object%20Reference :default "/Game/Gold_Store/Input/Controlls/VR_Teleport_Right.VR_Teleport_Right"))
  (bind _rightmotioncontroller (Variables|Default|GetRightMotionController))
  (bind _widgetinteractionright (Variables|Default|GetWidgetInteractionRight))
  (:Triggered
    (if (Variables|Default|GetCan%20Teleport%20Right)
      (CallFunction|VisibleTeleportRing (Transformation|GetWorldLocation _rightmotioncontroller) (Math|Vector|GetForwardVector _rightmotioncontroller))))
  (:Started
    (if (Components|Activation|IsActive _widgetinteractionright)
      (Class|WidgetInteractionComponent|PressPointerKey _widgetinteractionright "LeftMouseButton")
      (Class|WidgetInteractionComponent|ReleasePointerKey _widgetinteractionright "LeftMouseButton")
      (else
        (Variables|Default|SetCan%20Teleport%20Right true)
        (Variables|Default|SetCan%20Teleport%20Left false))))
  (:Completed
    (if (Variables|Default|GetCan%20Teleport%20Right)
      (CallFunction|Teleport&ClearArc)
      (Variables|Default|SetCan%20Teleport%20Right false))))

(event Input|EnhancedActionEvents|EnhancedInputActionVR_Teleport_Left
  (params (ActionValue :type Boolean) (ElapsedSeconds :type Float%20%28double-precision%29) (TriggeredSeconds :type Float%20%28double-precision%29) (InputAction :type Input%20Action%20Object%20Reference :default "/Game/Gold_Store/Input/Controlls/VR_Teleport_Left.VR_Teleport_Left"))
  (bind _leftmotioncontroller (Variables|Default|GetLeftMotionController))
  (bind _widgetinteractionleft (Variables|Default|GetWidgetInteractionLeft))
  (:Triggered
    (if (Variables|Default|GetCan%20Teleport%20Left)
      (CallFunction|VisibleTeleportRing (Transformation|GetWorldLocation _leftmotioncontroller) (Math|Vector|GetForwardVector _leftmotioncontroller))))
  (:Started
    (if (Components|Activation|IsActive _widgetinteractionleft)
      (Class|WidgetInteractionComponent|PressPointerKey _widgetinteractionleft "LeftMouseButton")
      (Class|WidgetInteractionComponent|ReleasePointerKey _widgetinteractionleft "LeftMouseButton")
      (else
        (Variables|Default|SetCan%20Teleport%20Left true)
        (Variables|Default|SetCan%20Teleport%20Right false))))
  (:Completed
    (if (Variables|Default|GetCan%20Teleport%20Left)
      (CallFunction|Teleport&ClearArc)
      (Variables|Default|SetCan%20Teleport%20Left false))))

(event Input|EnhancedActionEvents|EnhancedInputActionVR_Jump
  (params (ActionValue :type Boolean) (ElapsedSeconds :type Float%20%28double-precision%29) (TriggeredSeconds :type Float%20%28double-precision%29) (InputAction :type Input%20Action%20Object%20Reference :default "/Game/Gold_Store/Input/Controlls/VR_Jump.VR_Jump"))
  (:Started
    (Character|Jump))
  (:Completed
    (Character|StopJumping)))

(event Input|EnhancedActionEvents|EnhancedInputActionVRGrabLeft
  (params (ActionValue :type Boolean) (ElapsedSeconds :type Float%20%28double-precision%29) (TriggeredSeconds :type Float%20%28double-precision%29) (InputAction :type Input%20Action%20Object%20Reference :default "/Game/Gold_Store/Input/Controlls/VRGrabLeft.VRGrabLeft"))
  (:Started
    (Utilities|IsValid (Variables|Default|GetGrabComponet)
      (:Is%20Not%20Valid
        (bind _vrgrabcomponent (CallFunction|GetGrabComponent (Variables|Default|GetLeftHand) "middle_01_l"))
        (Utilities|IsValid _vrgrabcomponent
          (:Is%20Valid
            (bind _isheld (Default|TryGrab _vrgrabcomponent (Variables|Default|GetLeftMotionController)))
            (if _isheld
              (bind _output_get (Variables|Default|SetLeftHandHeldComponent _vrgrabcomponent))
              (Variables|Default|SetGrabComponet _output_get)
              (Components|Activation|Activate (Variables|Default|GetWidgetInteractionRight) false)
              (Rendering|SetVisibility (Variables|Default|GetXRDeviceVisualizationRight) true false)
              (Rendering|SetVisibility (Variables|Default|GetRightHand) false false)))))))
  (:Completed
    (bind _lefthandheldcomponent (Variables|Default|GetLeftHandHeldComponent)
      (:then
        (bind _breleased (Default|TryRelease _lefthandheldcomponent))
        (if _breleased
          (Variables|Default|SetLeftHandHeldComponent 0)
          (Variables|Default|SetGrabComponet 0)
          (Components|Activation|Deactivate (Variables|Default|GetWidgetInteractionRight))
          (Rendering|SetVisibility (Variables|Default|GetXRDeviceVisualizationRight) false false)
          (Rendering|SetVisibility (Variables|Default|GetRightHand) true false)))
      (:else))))

(event Input|EnhancedActionEvents|EnhancedInputActionVRGrabRight
  (params (ActionValue :type Boolean) (ElapsedSeconds :type Float%20%28double-precision%29) (TriggeredSeconds :type Float%20%28double-precision%29) (InputAction :type Input%20Action%20Object%20Reference :default "/Game/Gold_Store/Input/Controlls/VRGrabRight.VRGrabRight"))
  (:Started
    (Utilities|IsValid (Variables|Default|GetGrabComponet)
      (:Is%20Not%20Valid
        (bind _vrgrabcomponent (CallFunction|GetGrabComponent (Variables|Default|GetRightHand) "middle_01_r"))
        (Utilities|IsValid _vrgrabcomponent
          (:Is%20Valid
            (bind _isheld (Default|TryGrab _vrgrabcomponent (Variables|Default|GetRightMotionController)))
            (if _isheld
              (bind _output_get (Variables|Default|SetRightHandHeldComponent _vrgrabcomponent))
              (Variables|Default|SetGrabComponet _output_get)
              (Components|Activation|Activate (Variables|Default|GetWidgetInteractionLeft) false)
              (Rendering|SetVisibility (Variables|Default|GetXRDeviceVisualizationLeft) true false)
              (Rendering|SetVisibility (Variables|Default|GetLeftHand) false false)))))))
  (:Completed
    (bind _righthandheldcomponent (Variables|Default|GetRightHandHeldComponent)
      (:then
        (bind _breleased (Default|TryRelease _righthandheldcomponent))
        (if _breleased
          (Variables|Default|SetRightHandHeldComponent 0)
          (Variables|Default|SetGrabComponet 0)
          (Components|Activation|Deactivate (Variables|Default|GetWidgetInteractionLeft))
          (Rendering|SetVisibility (Variables|Default|GetXRDeviceVisualizationLeft) false false)
          (Rendering|SetVisibility (Variables|Default|GetLeftHand) true false)))
      (:else))))

(event EventBeginPlay
  (bind _returnvalue (Game|GetPlayerController 0))
  (bind _returnvalue_2 (PlayerController|LocalPlayerSubsystems|GetEnhancedInputLocalPlayerSubsystem _returnvalue))
  (Class|HeadMountedDisplayFunctionLibrary|SetTrackingOrigin "Stage")
  (Input|AddMappingContext _returnvalue_2 "/Game/Gold_Store/Input/VR_Defualt_Controller.VR_Defualt_Controller" 10 "(bIgnoreAllPressedKeysUntilRelease=True,bForceImmediately=False,bNotifyUserSettings=False)")
  (Input|AddMappingContext _returnvalue_2 "/Game/Gold_Store/Input/VR_IMC_Hand_Animations.VR_IMC_Hand_Animations" 10 "(bIgnoreAllPressedKeysUntilRelease=True,bForceImmediately=False,bNotifyUserSettings=False)")
  (Input|AddMappingContext _returnvalue_2 "/Game/Gold_Store/Input/VR_Grab_Teleport.VR_Grab_Teleport" 10 "(bIgnoreAllPressedKeysUntilRelease=True,bForceImmediately=False,bNotifyUserSettings=False)"))

(event Input|EnhancedActionEvents|EnhancedInputActionVR_IA_Hand_Grasp_Right
  (params (ActionValue :type Float%20%28double-precision%29) (ElapsedSeconds :type Float%20%28double-precision%29) (TriggeredSeconds :type Float%20%28double-precision%29) (InputAction :type Input%20Action%20Object%20Reference :default "/Game/Gold_Store/Input/Controlls/VR_IA_Hand_Grasp_Right.VR_IA_Hand_Grasp_Right"))
  (bind _righthand (Variables|Default|GetRightHand))
  (bind _returnvalue (Components|SkeletalMesh|GetAnimInstance _righthand))
  ;[0.1031 0.1031 0.1031] Hand Animations
  (:Triggered
    (bind _asvr_abp_mannequins_xr (Utilities|Casting|CastToVR_ABP_MannequinsXR _returnvalue))
    (Variables|/Game/Characters/MannequinsXR/Meshes/VR_ABP_MannequinsXR.VR_ABP_MannequinsXR_C|SetPoseAlphaGrasp _asvr_abp_mannequins_xr ActionValue))
  (:Canceled
    (bind _asvr_abp_mannequins_xr_2 (Utilities|Casting|CastToVR_ABP_MannequinsXR _returnvalue :!label _label))
    (Variables|/Game/Characters/MannequinsXR/Meshes/VR_ABP_MannequinsXR.VR_ABP_MannequinsXR_C|SetPoseAlphaGrasp _asvr_abp_mannequins_xr_2 0.0))
  (:Completed
    (goto _label)))

(event Input|EnhancedActionEvents|EnhancedInputActionVR_IA_Hand_Point_Right
  (params (ActionValue :type Float%20%28double-precision%29) (ElapsedSeconds :type Float%20%28double-precision%29) (TriggeredSeconds :type Float%20%28double-precision%29) (InputAction :type Input%20Action%20Object%20Reference :default "/Game/Gold_Store/Input/Controlls/VR_IA_Hand_Point_Right.VR_IA_Hand_Point_Right"))
  (bind _righthand (Variables|Default|GetRightHand))
  (bind _returnvalue (Components|SkeletalMesh|GetAnimInstance _righthand))
  ;[0.1031 0.1031 0.1031] Hand Animations
  (:Started
    (bind _asvr_abp_mannequins_xr (Utilities|Casting|CastToVR_ABP_MannequinsXR _returnvalue :!label _label))
    (Variables|/Game/Characters/MannequinsXR/Meshes/VR_ABP_MannequinsXR.VR_ABP_MannequinsXR_C|SetPoseAlphaPoint _asvr_abp_mannequins_xr 1.0))
  (:Canceled
    (goto _label))
  (:Completed
    (bind _asvr_abp_mannequins_xr_2 (Utilities|Casting|CastToVR_ABP_MannequinsXR _returnvalue))
    (Variables|/Game/Characters/MannequinsXR/Meshes/VR_ABP_MannequinsXR.VR_ABP_MannequinsXR_C|SetPoseAlphaPoint _asvr_abp_mannequins_xr_2 0.0)))

(event Input|EnhancedActionEvents|EnhancedInputActionVR_IA_Hand_Point_Left
  (params (ActionValue :type Float%20%28double-precision%29) (ElapsedSeconds :type Float%20%28double-precision%29) (TriggeredSeconds :type Float%20%28double-precision%29) (InputAction :type Input%20Action%20Object%20Reference :default "/Game/Gold_Store/Input/Controlls/VR_IA_Hand_Point_Left.VR_IA_Hand_Point_Left"))
  (bind _lefthand (Variables|Default|GetLeftHand))
  (bind _returnvalue (Components|SkeletalMesh|GetAnimInstance _lefthand))
  ;[0.1031 0.1031 0.1031] Hand Animations
  (:Started
    (bind _asvr_abp_mannequins_xr (Utilities|Casting|CastToVR_ABP_MannequinsXR _returnvalue :!label _label))
    (Variables|/Game/Characters/MannequinsXR/Meshes/VR_ABP_MannequinsXR.VR_ABP_MannequinsXR_C|SetPoseAlphaPoint _asvr_abp_mannequins_xr 1.0))
  (:Canceled
    (goto _label))
  (:Completed
    (bind _asvr_abp_mannequins_xr_2 (Utilities|Casting|CastToVR_ABP_MannequinsXR _returnvalue))
    (Variables|/Game/Characters/MannequinsXR/Meshes/VR_ABP_MannequinsXR.VR_ABP_MannequinsXR_C|SetPoseAlphaPoint _asvr_abp_mannequins_xr_2 0.0)))

(event Input|EnhancedActionEvents|EnhancedInputActionVR_IA_Hand_Grasp_Left
  (params (ActionValue :type Float%20%28double-precision%29) (ElapsedSeconds :type Float%20%28double-precision%29) (TriggeredSeconds :type Float%20%28double-precision%29) (InputAction :type Input%20Action%20Object%20Reference :default "/Game/Gold_Store/Input/Controlls/VR_IA_Hand_Grasp_Left.VR_IA_Hand_Grasp_Left"))
  (bind _lefthand (Variables|Default|GetLeftHand))
  (bind _returnvalue (Components|SkeletalMesh|GetAnimInstance _lefthand))
  ;[0.1031 0.1031 0.1031] Hand Animations
  (:Triggered
    (bind _asvr_abp_mannequins_xr (Utilities|Casting|CastToVR_ABP_MannequinsXR _returnvalue))
    (Variables|/Game/Characters/MannequinsXR/Meshes/VR_ABP_MannequinsXR.VR_ABP_MannequinsXR_C|SetPoseAlphaGrasp _asvr_abp_mannequins_xr ActionValue))
  (:Canceled
    (bind _asvr_abp_mannequins_xr_2 (Utilities|Casting|CastToVR_ABP_MannequinsXR _returnvalue :!label _label))
    (Variables|/Game/Characters/MannequinsXR/Meshes/VR_ABP_MannequinsXR.VR_ABP_MannequinsXR_C|SetPoseAlphaGrasp _asvr_abp_mannequins_xr_2 0.0))
  (:Completed
    (goto _label)))

(event OnComponentActivated(WidgetInteractionLeft)
  (params (Component :type Actor%20Component%20Object%20Reference) (bReset :type Boolean))
  (Rendering|SetVisibility (Variables|Default|GetLeftWidgetCylinder) true false)
  (bind _returnvalue (Utilities|Time|SetTimerbyEvent (delegate Custom|Left%20Widget%20Interaction%20Event) 0.0001 true true))
  (Variables|Default|SetLeft%20Widget%20Timer _returnvalue))

(event OnComponentDeactivated(WidgetInteractionLeft)
  (params (Component :type Actor%20Component%20Object%20Reference))
  (Utilities|Time|ClearandInvalidateTimerbyHandle (Variables|Default|GetLeft%20Widget%20Timer))
  (Rendering|SetVisibility (Variables|Default|GetLeftWidgetSphere) false false))

(event OnComponentActivated(WidgetInteractionRight)
  (params (Component :type Actor%20Component%20Object%20Reference) (bReset :type Boolean))
  (Rendering|SetVisibility (Variables|Default|GetRightWidgetCylinder) true false)
  (bind _returnvalue (Utilities|Time|SetTimerbyEvent (delegate Custom|Right%20Widget%20Interaction%20Event) 0.0001 true true))
  (Variables|Default|SetRight%20Widget%20Timer _returnvalue))

(event OnComponentDeactivated(WidgetInteractionRight)
  (params (Component :type Actor%20Component%20Object%20Reference))
  (Utilities|Time|ClearandInvalidateTimerbyHandle (Variables|Default|GetRight%20Widget%20Timer))
  (Rendering|SetVisibility (Variables|Default|GetRightWidgetSphere) false false))

(event Custom|Right%20Widget%20Interaction%20Event
  (bind _widgetinteractionright (Variables|Default|GetWidgetInteractionRight))
  (bind _rightwidgetsphere (Variables|Default|GetRightWidgetSphere))
  (bind _rightwidgetcylinder (Variables|Default|GetRightWidgetCylinder))
  (bind _returnvalue (Transformation|GetWorldLocation _widgetinteractionright))
  (bind (_outhit _returnvalue_2) (Collision|LineTraceForObjects _returnvalue (+ _returnvalue (* (Math|Vector|GetForwardVector (Transformation|GetWorldRotation _widgetinteractionright)) 500)) (Utilities|Array|MakeArray "ObjectTypeQuery2") false (Utilities|Array|MakeArray self) "None"))
  (if _returnvalue_2
    (Transformation|SetRelativeScale3D _rightwidgetcylinder (Math|Vector|MakeVector 0.005 0.005 (/ (Math|Vector|VectorLength (- (.TraceStart (Collision|BreakHitResult _outhit)) (.Location (Collision|BreakHitResult _outhit)))) 1e+02)))
    (Rendering|SetVisibility _rightwidgetsphere true false)
    (Transformation|SetWorldLocation _rightwidgetsphere (.Location (Collision|BreakHitResult _outhit)) false true)
    (else
      (Transformation|SetRelativeScale3D _rightwidgetcylinder (Math|Vector|MakeVector 0.005 0.005 5.0))
      (Rendering|SetVisibility (Variables|Default|GetRightWidgetSphere) false false))))

(event Custom|Left%20Widget%20Interaction%20Event
  (bind _widgetinteractionleft (Variables|Default|GetWidgetInteractionLeft))
  (bind _leftwidgetsphere (Variables|Default|GetLeftWidgetSphere))
  (bind _leftwidgetcylinder (Variables|Default|GetLeftWidgetCylinder))
  (bind _returnvalue (Transformation|GetWorldLocation _widgetinteractionleft))
  (bind (_outhit _returnvalue_2) (Collision|LineTraceForObjects _returnvalue (+ _returnvalue (* (Math|Vector|GetForwardVector (Transformation|GetWorldRotation _widgetinteractionleft)) 500)) (Utilities|Array|MakeArray "ObjectTypeQuery2") false (Utilities|Array|MakeArray self) "None"))
  (if _returnvalue_2
    (Transformation|SetRelativeScale3D _leftwidgetcylinder (Math|Vector|MakeVector 0.005 0.005 (/ (Math|Vector|VectorLength (- (.TraceStart (Collision|BreakHitResult _outhit)) (.Location (Collision|BreakHitResult _outhit)))) 1e+02)))
    (Rendering|SetVisibility _leftwidgetsphere true false)
    (Transformation|SetWorldLocation _leftwidgetsphere (.Location (Collision|BreakHitResult _outhit)) false true)
    (else
      (Transformation|SetRelativeScale3D _leftwidgetcylinder (Math|Vector|MakeVector 0.005 0.005 5.0))
      (Rendering|SetVisibility (Variables|Default|GetLeftWidgetSphere) false false))))

(fn ConstructionScript)

(fn VisibleTeleportRing
  (params (Start%20Pos :type Vector) (End%20Pos :type Vector))
  (bind _trace_line (Variables|Default|GetTrace%20Line))
  (bind (_outhit _outpathpositions _outlasttracedestination _returnvalue) (Class|GameplayStatics|BlueprintPredictProjectilePathbyTraceChannel Start%20Pos (* End%20Pos 5e+02) true 5.0 "ECC_WorldStatic" false (CallFunction|GetActorstoIgnore) "None"))
  (if _returnvalue
    (LocalVariables|SetPath%20of%20Line _outpathpositions)
    (for _array_element _trace_line
      (Components|DestroyComponent _array_element))
    (Utilities|Array|Clear _trace_line)
    (for _index (range 1 (- (Utilities|Array|Length (LocalVariables|GetPath%20of%20Line)) 2))
      (bind _returnvalue_2 (AddComponent|AddStaticMeshComponent true (Math|Transform|MakeTransform (Utilities|Array|Get(acopy) (LocalVariables|GetPath%20of%20Line) (- _index 1)) "0, 0, 0" "0.025000,0.025000,0.025000")))
      (Utilities|Array|Add (Variables|Default|GetTrace%20Line) _returnvalue_2))
    (if (.ReturnValue (AI|Navigation|ProjectPointtoNavigation _outlasttracedestination 0 0 "0, 0, 0"))
      (bind _output_get (Variables|Default|SetTeleport%20Location (.ProjectedLocation (AI|Navigation|ProjectPointtoNavigation _outlasttracedestination 0 0 "0, 0, 0"))))
      (Transformation|SetWorldLocation (Variables|Default|GetRing) _output_get false true)
      (Rendering|SetVisibility (Variables|Default|GetRing) true false)
      (else
        (Variables|Default|SetTeleport%20Location (Transformation|GetActorLocation) :!label _label)
        (Rendering|SetVisibility (Variables|Default|GetRing) false false)))
    (else
      (goto _label))))

(fn Teleport&ClearArc
  (bind _trace_line (Variables|Default|GetTrace%20Line))
  (Transformation|SetActorLocation (Variables|Default|GetTeleport%20Location) false true)
  (for _array_element _trace_line
    (Components|DestroyComponent _array_element))
  (Utilities|Array|Clear _trace_line)
  (Rendering|SetVisibility (Variables|Default|GetRing) false false))

(fn GetGrabComponent
  (params (Motion%20Controller :type Skeletal%20Mesh%20Component%20Object%20Reference) (Socket%20Name :type Name))
  (bind _returnvalue (Transformation|GetWorldRotation Motion%20Controller))
  (bind _returnvalue_2 (Transformation|GetSocketLocation Motion%20Controller Socket%20Name))
  (bind _returnvalue_3 (Math|Vector|GetUpVector _returnvalue))
  (bind _returnvalue_4 (* _returnvalue_3 -6.0))
  (bind _returnvalue_5 (+ _returnvalue_4 _returnvalue_2))
  (bind (_outhit _returnvalue_6) (Collision|SphereTraceForObjects _returnvalue_5 _returnvalue_5 3.0 (Utilities|Array|MakeArray "ObjectTypeQuery4") false (Utilities|Array|MakeArray self) "None"))
  (if _returnvalue_6
    (return (Actor|GetComponentbyClass (.HitActor (Collision|BreakHitResult _outhit)) "/Game/Gold_Store/BluePrint/VRGrabComponent.VRGrabComponent_C"))
    (else
      (return 0))))

(fn GetActorstoIgnore
  (bind _grabcomponet (Variables|Default|GetGrabComponet))
  (bind _returnvalue (Components|GetOwner _grabcomponet))
  (Utilities|IsValid (Variables|Default|GetGrabComponet)
    (:Is%20Valid
      (Utilities|IsValid _returnvalue
        (:Is%20Valid
          (return (Utilities|Array|MakeArray self _returnvalue)))
        (:Is%20Not%20Valid
          _)))
    (:Is%20Not%20Valid
      _))
  (return (Utilities|Array|MakeArray self)))