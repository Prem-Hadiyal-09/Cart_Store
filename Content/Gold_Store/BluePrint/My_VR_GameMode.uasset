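; VR game mode for a store that manages the shopping cart as a map of product row names to quantities.
; It adds, decrements and clears items, and totals quantity and cost using prices from the Products_List data table.
; It fills the product widget on the item the VR character grabs and lists cart contents on the Counter's widget, which it finds at BeginPlay.
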(event EventBeginPlay
  (Utilities|FlowControl|Sequence
    (:then_0
      (bind _returnvalue (Actor|GetActorOfClass "/Game/Store/BP_Product_Base.BP_Product_Base_C"))
      (Variables|Default|SetProduct%20Base _returnvalue))
    (:then_1
      (bind _returnvalue_2 (Actor|GetActorOfClass "/Game/Store/Counter/Counter.Counter_C"))
      (Variables|Default|SetBP%20Counter _returnvalue_2))))

(fn ConstructionScript)

(fn IsCartEmpty
  (return (Utilities|Map|IsEmpty (Variables|Default|GetCart))))

(fn IsProductinCart
  (params (RowName :type Name))
  (return (Utilities|Map|Contains (Variables|Default|GetCart) RowName)))

(fn AddIteminCart
  (params (Row%20Name :type Name))
  (LocalVariables|SetKey Row%20Name)
  (if (.ReturnValue (Utilities|Map|Find (Variables|Default|GetCart) (LocalVariables|GetKey)))
    (bind _output_get (LocalVariables|SetQuantity (.Value (Utilities|Map|Find (Variables|Default|GetCart) (LocalVariables|GetKey)))))
    (Math|Integer|IncrementInt _output_get
      (:%20%20
        (Utilities|Map|Add (Variables|Default|GetCart) (LocalVariables|GetKey) (LocalVariables|GetQuantity))
        (return (LocalVariables|GetQuantity))))
    (else
      (Utilities|Map|Add (Variables|Default|GetCart) (LocalVariables|GetKey) 1))))

(fn RemoveItemfromCart
  (params (Row%20Name :type Name))
  (LocalVariables|SetKey Row%20Name)
  (if (.ReturnValue (Utilities|Map|Find (Variables|Default|GetCart) (LocalVariables|GetKey)))
    (bind _output_get (LocalVariables|SetProduct%20Qty (.Value (Utilities|Map|Find (Variables|Default|GetCart) (LocalVariables|GetKey)))))
    (if (> _output_get 0)
      (Math|Integer|DecrementInt (LocalVariables|GetProduct%20Qty)
        (:%20%20
          (Utilities|Map|Add (Variables|Default|GetCart) (LocalVariables|GetKey) (LocalVariables|GetProduct%20Qty))
          (return (LocalVariables|GetProduct%20Qty))))
      (else
        (Utilities|Map|Remove (Variables|Default|GetCart) (LocalVariables|GetKey))))))

(fn TotalCost
  (bind _keys (Utilities|Map|Keys (Variables|Default|GetCart)))
  (for _array_element _keys
    (bind _output_get (LocalVariables|SetRow%20Name _array_element))
    (bind _returnvalue (Utilities|GetDataTableRow "/Game/Store/Product/Products_List.Products_List" _output_get)
      (:then
        (LocalVariables|SetTotal%20Bill%20Amt (+ (* (.ProductCost (Utilities|Struct|BreakProduct_DATA _returnvalue)) (.Value (Utilities|Map|Find (Variables|Default|GetCart) (LocalVariables|GetRow%20Name)))) (LocalVariables|GetTotal%20Bill%20Amt))))))
  (return (LocalVariables|GetTotal%20Bill%20Amt)))

(fn TotalQuantityinCart
  (bind _values (Utilities|Map|Values (Variables|Default|GetCart)))
  (for _array_element _values
    (LocalVariables|SetTotal%20Qty (+ _array_element (LocalVariables|GetTotal%20Qty))))
  (return (LocalVariables|GetTotal%20Qty)))

(fn DisplayProductUI
  (params (Row%20Name :type Name))
  (bind _asvr_character (Utilities|Casting|CastToVR_Character (Game|GetPlayerCharacter 0)))
  (bind _asbp_product_base (Utilities|Casting|CastToBP_Product_Base (Components|GetOwner (Variables|/Game/Gold_Store/BluePrint/VR_Character.VR_Character_C|GetGrabComponet _asvr_character))))
  (bind _asproduct_ui (Utilities|Casting|CastToProduct_UI (UserInterface|GetWidget (Variables|/Game/Store/BP_Product_Base.BP_Product_Base_C|GetWidget _asbp_product_base))))
  (Default|SetProductUIText _asproduct_ui Row%20Name)
  (bind _is_product_avilable (CallFunction|IsProductinCart Row%20Name))
  (Default|HideAddtoCartButton _asproduct_ui _is_product_avilable))

(fn DisplayCartUI
  (bind _keys (Utilities|Map|Keys (Variables|Default|GetCart)))
  (for _array_element _keys
    (bind _ascart_ui (Utilities|Casting|CastToCart_UI (UserInterface|GetWidget (Variables|/Game/Store/Counter/Counter.Counter_C|GetCounter%20Widget (Variables|Default|GetBP%20Counter)))))
    (Default|AddProducttoItemList _ascart_ui _array_element))
  (return))

(fn ClearCart
  (params (Row%20Name :type Name))
  (Utilities|Map|Remove (Variables|Default|GetCart) Row%20Name))