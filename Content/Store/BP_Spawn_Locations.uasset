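; BP_Spawn_Locations is a store spawn point that fills its child actor with a random product on BeginPlay.
; It picks a random row from the Products_List data table and sets the ChildActor class to that row's ProductClass.
; It then passes the row name through SetData to every BP_Product_Base actor in the world matching that class, not only its own child.
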(event EventBeginPlay
  (bind _outrownames (DataTable|GetDataTableRowNames "/Game/Store/Product/Products_List.Products_List"))
  (bind _output_get (Variables|Default|SetRow%20Name (.OutItem (Utilities|Array|Random _outrownames))))
  (bind _returnvalue (Utilities|GetDataTableRow "/Game/Store/Product/Products_List.Products_List" _output_get)
    (:then
      (ChildActorComponent|SetChildActorClass (Variables|Default|GetChildActor) (Utilities|Struct|BreakProduct_DATA _returnvalue))
      (bind _outactors (Actor|GetAllActorsOfClass "/Game/Store/BP_Product_Base.BP_Product_Base_C"))
      (bind _filteredarray (Utilities|Array|FilterArray _outactors (Utilities|Struct|BreakProduct_DATA _returnvalue)))
      (for _array_element _filteredarray
        (Default|SetData (.AsBP%20Product%20Base (Utilities|Casting|CastToBP_Product_Base _array_element)) (Variables|Default|GetRow%20Name))))))

(fn ConstructionScript)